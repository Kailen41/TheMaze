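; Actor component that handles crouch and jump movement for the player character, BP_Player.
; On BeginPlay it caches the first player character cast to BP_Player.
; Crouch events switch max walk speed between crouch and walk values, tell the player to shorten or lengthen its capsule, and track an IsCrouching flag.
; Jump events forward directly to the character's Jump and StopJumping.
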(event `self.ReceiveBeginPlay`
  (bind _asbp_player (cast `/Game/_Main/Blueprints/Actors/Player/BP_Player` (`GameplayStatics.GetPlayerCharacter` 0)))
  (set `self.Player_REF` _asbp_player))

(event `StartCrouch`
  (bind _player_ref (`self.Player_REF`))
  (set `CharacterMovementComponent.MaxWalkSpeed` (`self.CrouchSpeed`) (`Character.CharacterMovement` _player_ref))
  (`/Game/_Main/Blueprints/Actors/Player/BP_Player.ShortenCapsule` _player_ref)
  (set `self.IsCrouching?` true))

(event `EndCrouch`
  (bind _player_ref (`self.Player_REF`))
  (set `CharacterMovementComponent.MaxWalkSpeed` (`self.WalkSpeed`) (`Character.CharacterMovement` _player_ref))
  (`/Game/_Main/Blueprints/Actors/Player/BP_Player.LengthenCapsule` _player_ref)
  (set `self.IsCrouching?` false))

(event `Jumping`
  (`Character.Jump` (`self.Player_REF`)))

(event `EndJumping`
  (`Character.StopJumping` (`self.Player_REF`)))