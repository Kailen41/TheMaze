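; Flashlight component that toggles the player's light with a click sound and manages its battery life.
; Initialization caches the player and its Flashlight light; switching on requires charge above the minimum and starts a looping timer that drains the battery.
; Battery changes are clamped and remapped to the light's IES brightness scale, and an empty battery hides the light and stops the timer.
; A separate function adds charge and refreshes brightness.
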(event `self.ReceiveTick`
  (params (DeltaSeconds :type "Float (single-precision)")))

(fn `f_AddBtteryLife`
  (params (Amount :type "Float (double-precision)"))
  (set `self.CurrentBatteryLevel` (`KismetMathLibrary.FClamp` (+ (`self.CurrentBatteryLevel`) Amount) (`self.MinBatteryLevel`) (`self.MaxBatteryLevel`)))
  (`self.f_SetIntensity`))

(fn `f_DepleteBatteryLife`
  (bind _output_get (set `self.CurrentBatteryLevel` (`KismetMathLibrary.FClamp` (- (`self.CurrentBatteryLevel`) (`self.DepletionAmount`)) (`self.MinBatteryLevel`) (`self.MaxBatteryLevel`))))
  (`self.f_SetIntensity`)
  (if (<= _output_get (`self.MinBatteryLevel`))
    (`SceneComponent.SetVisibility` (`self.FlashlightLIght`) false false)
    (`KismetSystemLibrary.K2_ClearTimer` null "f_DepleteBatteryLife")))

(fn `f_Initialize`
  (params (Player :type "/Game/_Main/Blueprints/Actors/Player/BP_Player Object Reference"))
  (bind _output_get (set `self.Player_REF` Player))
  (set `self.FlashlightLIght` (`/Game/_Main/Blueprints/Actors/Player/BP_Player.Flashlight` _output_get)))

(fn `f_SetIntensity`
  (`LightComponent.SetIESBrightnessScale` (`self.FlashlightLIght`) (`KismetMathLibrary.MapRangeClamped` (`self.CurrentBatteryLevel`) (`self.MinBatteryLevel`) 20.0 0.0 0.5)))

(fn `f_ToggleFlashlight`
  (bind _flashlightlight (`self.FlashlightLIght`))
  (`GameplayStatics.PlaySound2D` "/Game/_Main/Audio/SFX/ClickSound.ClickSound" 1.0 1.0 0.0 null null)
  (if (`SceneComponent.bVisible` _flashlightlight)
    (`SceneComponent.SetVisibility` _flashlightlight false false)
    (`KismetSystemLibrary.K2_ClearTimer` null "f_DepleteBatteryLife")
    (elif (> (`self.CurrentBatteryLevel`) (`self.MinBatteryLevel`))
      (`self.f_SetIntensity`)
      (`SceneComponent.SetVisibility` _flashlightlight true false)
      (`KismetSystemLibrary.K2_SetTimer` null "f_DepleteBatteryLife" (`self.DepletionSpeed`) true))))