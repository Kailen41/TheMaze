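; Game mode for the maze game that manages the HUD and the lose sequence.
; On BeginPlay it creates the HUD widget and adds it to the viewport.
; LoseEvent disables player input, fades the camera to a held red tint and removes the HUD, then after a short delay shows the lose screen with UI-only input and a visible cursor.
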(event `self.ReceiveBeginPlay`
  (bind _returnvalue (`|CreateWidget` "/Game/_Main/UI/UMG/W_HUD.W_HUD_C"))
  (bind _output_get (set `self.HUD_Ref` _returnvalue))
  (`UserWidget.AddToViewport` _output_get 0))

(event `LoseEvent`
  (bind _returnvalue (`GameplayStatics.GetPlayerController` 0))
  (`self.DisableInput` (`GameplayStatics.GetPlayerCharacter` 0) (`GameplayStatics.GetPlayerController` 0))
  (`PlayerCameraManager.StartCameraFade` (`GameplayStatics.GetPlayerCameraManager` 0) 0.0 0.8 2.0 (struct :`R` 1.0 :`A` 1.0) false true)
  (`Widget.RemoveFromParent` (`self.HUD_Ref`))
  (`KismetSystemLibrary.Delay` 2.0)
  (bind _returnvalue_2 (`|CreateWidget` "/Game/_Main/UI/UMG/W_LoseScreen.W_LoseScreen_C"))
  (`UserWidget.AddToViewport` _returnvalue_2 0)
  (`WidgetBlueprintLibrary.SetInputMode_UIOnlyEx` _returnvalue _returnvalue_2)
  (set `PlayerController.bShowMouseCursor` true _returnvalue))

(fn `UserConstructionScript`)