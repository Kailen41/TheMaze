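; BP_KeyPlatform is a maze pickup platform whose key mesh, shown to the player as a statue, can be collected.
; A trigger volume enables input and shows a HUD prompt while the player overlaps it, then disables input and clears it on exit.
; The interaction input destroys the mesh, increments the player's key count, refreshes the statue HUD via the game mode and plays a pickup sound.
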(event `EnhancedInput|/Game/_Main/Blueprints/Actors/Player/Input/Actions/IA_Interaction`
  (params (ActionValue :type Boolean) (ElapsedSeconds :type "Float (double-precision)") (TriggeredSeconds :type "Float (double-precision)") (InputAction :type "InputAction Object Reference" :default "/Game/_Main/Blueprints/Actors/Player/Input/Actions/IA_Interaction.IA_Interaction"))
  (bind _keymesh (`self.KeyMesh`))
  (:`Started`
    (`/Engine/EditorBlueprintResources/StandardMacros.IsValid` _keymesh
      (:`Is Valid`
        (`ActorComponent.K2_DestroyComponent` _keymesh)
        (bind _asbp_player (cast `/Game/_Main/Blueprints/Actors/Player/BP_Player` (`GameplayStatics.GetPlayerCharacter` 0)))
        (`/Engine/EditorBlueprintResources/StandardMacros.IncrementInt` (`/Game/_Main/Blueprints/Actors/Player/BP_Player.NumberOfKeys` _asbp_player)
          (:`  `
            (bind _asgm_maze_game_mode (cast `/Game/_Main/Blueprints/BaseClass/GM_MazeGameMode` (`GameplayStatics.GetGameMode`)))
            (`/Game/_Main/UI/UMG/W_HUD.UpdateStatues` (`/Game/_Main/Blueprints/BaseClass/GM_MazeGameMode.HUD_Ref` _asgm_maze_game_mode))
            (bind _asgm_maze_game_mode_2 (cast `/Game/_Main/Blueprints/BaseClass/GM_MazeGameMode` (`GameplayStatics.GetGameMode`)))
            (bind _hud_ref (`/Game/_Main/Blueprints/BaseClass/GM_MazeGameMode.HUD_Ref` _asgm_maze_game_mode_2))
            (set `/Game/_Main/UI/UMG/W_HUD.Message` "" _hud_ref)
            (`/Game/_Main/UI/UMG/W_HUD.UpdateMessage` _hud_ref)
            (`GameplayStatics.PlaySoundAtLocation` "/Engine/VREditor/Sounds/UI/Object_PickUp.Object_PickUp" (`self.K2_GetActorLocation` (`GameplayStatics.GetPlayerCharacter` 0)) (struct) 1.0 1.0 0.0 null null null null)))))))

(event `self.TriggerVolume.OnComponentBeginOverlap`
  (params (OverlappedComponent :type "PrimitiveComponent Object Reference") (OtherActor :type "Actor Object Reference") (OtherComp :type "PrimitiveComponent Object Reference") (OtherBodyIndex :type Integer) (bFromSweep :type Boolean) (SweepResult :type "HitResult Structure (by ref)"))
  (if (`self.ActorHasTag` OtherActor "Player")
    (`self.EnableInput` (`GameplayStatics.GetPlayerController` 0))
    (`/Engine/EditorBlueprintResources/StandardMacros.IsValid` (`self.KeyMesh`)
      (:`Is Valid`
        (bind _asgm_maze_game_mode (cast `/Game/_Main/Blueprints/BaseClass/GM_MazeGameMode` (`GameplayStatics.GetGameMode`)))
        (bind _hud_ref (`/Game/_Main/Blueprints/BaseClass/GM_MazeGameMode.HUD_Ref` _asgm_maze_game_mode))
        (set `/Game/_Main/UI/UMG/W_HUD.Message` "Press 'E' to pick up statue." _hud_ref)
        (`/Game/_Main/UI/UMG/W_HUD.UpdateMessage` _hud_ref)))))

(event `self.TriggerVolume.OnComponentEndOverlap`
  (params (OverlappedComponent :type "PrimitiveComponent Object Reference") (OtherActor :type "Actor Object Reference") (OtherComp :type "PrimitiveComponent Object Reference") (OtherBodyIndex :type Integer))
  (if (`self.ActorHasTag` OtherActor "Player")
    (`self.DisableInput` (`GameplayStatics.GetPlayerController` 0))
    (bind _asgm_maze_game_mode (cast `/Game/_Main/Blueprints/BaseClass/GM_MazeGameMode` (`GameplayStatics.GetGameMode`)))
    (bind _hud_ref (`/Game/_Main/Blueprints/BaseClass/GM_MazeGameMode.HUD_Ref` _asgm_maze_game_mode))
    (set `/Game/_Main/UI/UMG/W_HUD.Message` "" _hud_ref)
    (`/Game/_Main/UI/UMG/W_HUD.UpdateMessage` _hud_ref)))

(fn `UserConstructionScript`)