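; BP_Door is a maze door that the player opens by spending a key, shown to them as a statue.
; Overlapping its trigger while it is closed shows a HUD prompt and, if the player holds a key, enables input on the door; leaving clears both.
; Interacting decrements the key count, updates the HUD, attaches a key mesh and runs a timeline that moves key and door with sound, then marks it open.
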(event `self.TriggerVolume.OnComponentBeginOverlap`
  (params (OverlappedComponent :type "PrimitiveComponent Object Reference") (OtherActor :type "Actor Object Reference") (OtherComp :type "PrimitiveComponent Object Reference") (OtherBodyIndex :type Integer) (bFromSweep :type Boolean) (SweepResult :type "HitResult Structure (by ref)"))
  (if (`self.ActorHasTag` OtherActor "Player")
    (if (not (`self.IsOpen?`))
      (bind _asbp_player (cast `/Game/_Main/Blueprints/Actors/Player/BP_Player` (`GameplayStatics.GetPlayerCharacter` 0)))
      (if (> (`/Game/_Main/Blueprints/Actors/Player/BP_Player.NumberOfKeys` _asbp_player) 0)
        (`self.EnableInput` (`GameplayStatics.GetPlayerController` 0))
        (bind _asgm_maze_game_mode (cast `/Game/_Main/Blueprints/BaseClass/GM_MazeGameMode` (`GameplayStatics.GetGameMode`)))
        (bind _hud_ref (`/Game/_Main/Blueprints/BaseClass/GM_MazeGameMode.HUD_Ref` _asgm_maze_game_mode))
        (set `/Game/_Main/UI/UMG/W_HUD.Message` "Press 'E' to open door." _hud_ref)
        (`/Game/_Main/UI/UMG/W_HUD.UpdateMessage` _hud_ref)
        (else
          (bind _asgm_maze_game_mode_2 (cast `/Game/_Main/Blueprints/BaseClass/GM_MazeGameMode` (`GameplayStatics.GetGameMode`)))
          (bind _hud_ref_2 (`/Game/_Main/Blueprints/BaseClass/GM_MazeGameMode.HUD_Ref` _asgm_maze_game_mode_2))
          (set `/Game/_Main/UI/UMG/W_HUD.Message` "Door requires a statue to open." _hud_ref_2)
          (`/Game/_Main/UI/UMG/W_HUD.UpdateMessage` _hud_ref_2))))))

(event `self.TriggerVolume.OnComponentEndOverlap`
  (params (OverlappedComponent :type "PrimitiveComponent Object Reference") (OtherActor :type "Actor Object Reference") (OtherComp :type "PrimitiveComponent Object Reference") (OtherBodyIndex :type Integer))
  (if (`self.ActorHasTag` OtherActor "Player")
    (`self.DisableInput` (`GameplayStatics.GetPlayerController` 0))
    (bind _asgm_maze_game_mode (cast `/Game/_Main/Blueprints/BaseClass/GM_MazeGameMode` (`GameplayStatics.GetGameMode`)))
    (bind _hud_ref (`/Game/_Main/Blueprints/BaseClass/GM_MazeGameMode.HUD_Ref` _asgm_maze_game_mode))
    (set `/Game/_Main/UI/UMG/W_HUD.Message` "" _hud_ref)
    (`/Game/_Main/UI/UMG/W_HUD.UpdateMessage` _hud_ref)))

(event `EnhancedInput|/Game/_Main/Blueprints/Actors/Player/Input/Actions/IA_Interaction`
  (params (ActionValue :type Boolean) (ElapsedSeconds :type "Float (double-precision)") (TriggeredSeconds :type "Float (double-precision)") (InputAction :type "InputAction Object Reference" :default "/Game/_Main/Blueprints/Actors/Player/Input/Actions/IA_Interaction.IA_Interaction"))
  (:`Started`
    (bind _asbp_player (cast `/Game/_Main/Blueprints/Actors/Player/BP_Player` (`GameplayStatics.GetPlayerCharacter` 0)))
    (bind _numberofkeys (`/Game/_Main/Blueprints/Actors/Player/BP_Player.NumberOfKeys` _asbp_player))
    (if (> _numberofkeys 0)
      (`/Engine/EditorBlueprintResources/StandardMacros.DecrementInt` _numberofkeys
        (:`  `
          (bind _asgm_maze_game_mode (cast `/Game/_Main/Blueprints/BaseClass/GM_MazeGameMode` (`GameplayStatics.GetGameMode`)))
          (`/Game/_Main/UI/UMG/W_HUD.UpdateStatues` (`/Game/_Main/Blueprints/BaseClass/GM_MazeGameMode.HUD_Ref` _asgm_maze_game_mode))
          (bind _returnvalue (`AddComponent|NODE_AddStaticMeshComponent-0`))
          (bind _output_get (set `self.KeyMesh` _returnvalue))
          (`SceneComponent.K2_AttachToComponent` _output_get (`self.KeyLocation`) "None" "SnapToTarget" "SnapToTarget" "SnapToTarget" true)
          (`GameplayStatics.PlaySoundAtLocation` "/Game/_Main/Audio/SFX/DoorOpening_SFX.DoorOpening_SFX" (`self.K2_GetActorLocation`) (struct) 1.0 1.0 0.0 null null null null)
          (bind (_direction _dooralpha _keyalphay _keyalphaz) (`Timeline|DoorOpen` :!via `PlayFromStart`)
            (:`Update`
              (`SceneComponent.K2_SetRelativeLocation` (`self.KeyMesh`) (`KismetMathLibrary.MakeVector` 0.0 _keyalphay _keyalphaz) false false)
              (`SceneComponent.K2_SetRelativeLocation` (`self.Door`) (`KismetMathLibrary.MakeVector` 0.0 0.0 _dooralpha) false false)
              (bind _asgm_maze_game_mode_2 (cast `/Game/_Main/Blueprints/BaseClass/GM_MazeGameMode` (`GameplayStatics.GetGameMode`)))
              (bind _hud_ref (`/Game/_Main/Blueprints/BaseClass/GM_MazeGameMode.HUD_Ref` _asgm_maze_game_mode_2))
              (set `/Game/_Main/UI/UMG/W_HUD.Message` "" _hud_ref)
              (`/Game/_Main/UI/UMG/W_HUD.UpdateMessage` _hud_ref))
            (:`Finished`
              (set `self.IsOpen?` true))))))))

(fn `UserConstructionScript`)