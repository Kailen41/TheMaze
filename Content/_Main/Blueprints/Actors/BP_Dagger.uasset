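; BP_Dagger is a dagger actor that hurts and knocks back the player on contact.
; When its Collision overlaps BP_Player, it launches the player along its own velocity with a slight upward boost and applies damage.
; It then destroys itself and plays a hit sound at the player's location.
; Overlapping anything else destroys the dagger after a short delay.
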(event `self.Collision.OnComponentBeginOverlap`
  (params (OverlappedComponent :type "PrimitiveComponent Object Reference") (OtherActor :type "Actor Object Reference") (OtherComp :type "PrimitiveComponent Object Reference") (OtherBodyIndex :type Integer) (bFromSweep :type Boolean) (SweepResult :type "HitResult Structure (by ref)"))
  (bind _asbp_player (cast `/Game/_Main/Blueprints/Actors/Player/BP_Player` OtherActor)
    (:`then`
      (`Character.LaunchCharacter` _asbp_player (+ (`self.GetVelocity`) (0.0 0.0 100.0)) false false)
      (`GameplayStatics.ApplyDamage` _asbp_player 1.0)
      (`self.K2_DestroyActor`)
      (`GameplayStatics.PlaySoundAtLocation` "/Game/_Main/Audio/SFX/Hit_SFX.Hit_SFX" (`self.K2_GetActorLocation` (`GameplayStatics.GetPlayerCharacter` 0)) (struct) 1.0 1.0 0.0 null null null null))
    (:`CastFailed`
      (`KismetSystemLibrary.Delay` 2.0)
      (`self.K2_DestroyActor`))))

(fn `UserConstructionScript`)